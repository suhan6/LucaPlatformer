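; BP_MySplinePlatform is a platform that moves along a spline path, starting when play begins.
; A timeline's SplineDistance track is scaled by the spline length, and each update places the platform mesh at that world-space point without sweeping.
; The construction script applies a configurable static mesh and material to the platform.
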(event `self.ReceiveBeginPlay`
  (`self.PlatformStart`))

(event `PlatformStart`
  (bind _spline (`self.Spline`))
  (bind (_direction _splinedistance) (`Timeline|Motion Timeline`)
    (:`Update`
      (`SceneComponent.K2_SetWorldLocation` (`self.PlatformMesh`) (`SplineComponent.GetLocationAtDistanceAlongSpline` _spline (* _splinedistance (`SplineComponent.GetSplineLength` _spline)) "World") false false))))

(fn `UserConstructionScript`
  (bind _platformmesh (`self.PlatformMesh`))
  (`StaticMeshComponent.SetStaticMesh` _platformmesh (`self.Platform Mesh`))
  (`PrimitiveComponent.SetMaterial` _platformmesh 0 (`self.Material`)))